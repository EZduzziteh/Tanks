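; Player tank Blueprint that handles aim input by rotating a gimbal and spring arm.
; On BeginPlay it passes its Barrel component to SetBarrelReference.
; The AimAzimuth axis yaws AzimuthGimbol and AimElevation pitches SpringArm, both as frame-rate independent local rotations.
; Both axes scale by SensAimAzimuth, so elevation has no separate sensitivity here.
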(event EventBeginPlay
  (Class|PawnTankPlayer|SetBarrelReference (Variables|Default|Getbarrel)))

(event Input|AxisEvents|InputAxisAimAzimuth
  (params (AxisValue :type Float%20%28single-precision%29))
  (Transformation|AddLocalRotation (Variables|Default|Getazimuth%20gimbol) (Math|Rotator|MakeRotator 0.0 0.0 (* AxisValue (Utilities|Time|GetWorldDeltaSeconds) (Variables|Default|GetSens_Aim_Azimuth))) false false))

(event Input|AxisEvents|InputAxisAimElevation
  (params (AxisValue :type Float%20%28single-precision%29))
  (Transformation|AddLocalRotation (Variables|Default|GetSpringArm) (Math|Rotator|MakeRotator 0.0 (* AxisValue (Utilities|Time|GetWorldDeltaSeconds) (Variables|Default|GetSens_Aim_Azimuth)) 0.0) false false))

(fn ConstructionScript)